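; Interactable apartment door that swings open or closed, or shows a dialogue line when locked.
; Interact routes to DoorLocked, which picks dialogue by index, to an empty SpecialDoor event, or to ToggleDoor.
; ToggleDoor uses a dot product of player direction and door forward to choose the swing side, then timelines lerp the mesh yaw.
; A DoOnce blocks retriggering until each swing finishes.
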(event Custom|ToggleDoor
  (bind _defaultsceneroot (Variables|Default|GetDefaultSceneRoot))
  (Utilities|FlowControl|DoOnce false :!label _label
    (:Completed
      (if (Variables|Default|GetClosed?)
        (bind _output_get (Variables|Default|SetResultRotation (Math|Float|SelectFloat 0.0 -1.8e+02 (>= (Math|Vector|DotProduct (Math|Vector|Normalize (- (Transformation|GetWorldLocation _defaultsceneroot) (Transformation|GetActorLocation (Game|GetPlayerCharacter 0)))) (Math|Vector|GetForwardVector _defaultsceneroot)) 0.0))))
        (bind _newtrack_0 (Timeline|Timeline_0 PlayFromStart)
          (:Update
            (Transformation|SetRelativeRotation (Variables|Default|GetAppartment_Door1_WIP) (Math|Rotator|MakeRotator 0.0 0.0 (Math|Float|Lerp -9e+01 _output_get _newtrack_0)) false false))
          (:Finished
            (Variables|Default|SetClosed? false)
            (goto _label Reset)))
        (else
          (bind _newtrack_0_2 (Timeline|Timeline_1 PlayFromStart)
            (:Update
              (Transformation|SetRelativeRotation (Variables|Default|GetAppartment_Door1_WIP) (Math|Rotator|MakeRotator 0.0 0.0 (Math|Float|Lerp (Variables|Default|GetResultRotation) -9e+01 _newtrack_0_2)) false false))
            (:Finished
              (Variables|Default|SetClosed? true)
              (goto _label Reset))))))))

(event Custom|DoorLocked
  (switch int (Variables|Default|GetLockedDoorIndex)
    (:0
      (bind _returnvalue (UserInterface|CreateWidget "/Game/Player/UI/Shared/Dialogue.Dialogue_C"))
      (Variables|/Game/Player/UI/Shared/Dialogue.Dialogue_C|SetInputText _returnvalue "I gotta get ready first")
      (UserInterface|Viewport|AddtoViewport _returnvalue 0))))

(event Custom|SpecialDoor)

(fn ConstructionScript)

(fn Interact
  (if (Variables|Default|GetLocked?)
    (CallFunction|DoorLocked)
    (return true)
    (elif (Variables|Default|GetSpecialDoor?)
      (CallFunction|SpecialDoor)
      (return true)
      (else
        (CallFunction|ToggleDoor)
        (return true)))))