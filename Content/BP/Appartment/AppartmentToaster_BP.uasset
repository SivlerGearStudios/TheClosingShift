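; Interactable apartment toaster that turns bread held by the player into toast.
; Interact checks the player's ItemInHand: bread starts ToastBread, which empties the hand and sets Finished after a short delay, while anything else shows a dialogue hint.
; Once Finished, Interact hands the player a bread loaf mesh tagged as Toast and shows an eat prompt; the flag is never reset here.
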(event Custom|ToastBread
  (bind _asplayer (Utilities|Casting|CastToPlayer (Game|GetPlayerCharacter 0)))
  (Default|NullifyHand _asplayer)
  (Development|PrintString "Toasting")
  (Utilities|FlowControl|Delay 2.0)
  (Development|PrintString "Done!")
  (Variables|Default|SetFinished? true))

(fn ConstructionScript)

(fn Interact
  (if (Variables|Default|GetFinished?)
    (bind _asplayer (Utilities|Casting|CastToPlayer (Game|GetPlayerCharacter 0)))
    (Default|PickItem _asplayer "/Game/Meshes/CompletedAssets/Props/Appartment/BreadLoaf.BreadLoaf" (Math|Transform|MakeTransform "0, 0, 0" "0,180.000000, 0" "0.100000,0.100000,0.100000") "Toast")
    (bind _returnvalue (UserInterface|CreateWidget "/Game/Player/UI/Shared/InteractPrompt.InteractPrompt_C"))
    (Variables|/Game/Player/UI/Shared/InteractPrompt.InteractPrompt_C|SetInputText _returnvalue "Hit 'F' to eat")
    (UserInterface|Viewport|AddtoViewport _returnvalue 0)
    (else
      (bind _asplayer_2 (Utilities|Casting|CastToPlayer (Game|GetPlayerCharacter 0)))
      (if (Utilities|Enum|Equal(Enum) (Variables|/Game/Player/Player.Player_C|GetItemInHand _asplayer_2) "Bread")
        (CallFunction|ToastBread)
        (return true)
        (else
          (bind _returnvalue_2 (UserInterface|CreateWidget "/Game/Player/UI/Shared/Dialogue.Dialogue_C"))
          (Variables|/Game/Player/UI/Shared/Dialogue.Dialogue_C|SetInputText _returnvalue_2 "Gonna need some bread first")
          (UserInterface|Viewport|AddtoViewport _returnvalue_2 0)
          (return true))))))