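; CCTV monitor interactable in the restaurant that moves the player's view from first person to a fixed camera view.
; Interacting calls the player's PossessCamera, snaps the monitor's camera to the first-person camera's transform and switches the view target to it.
; After a short delay, two timelines lerp location and rotation to hardcoded values, and Active is set when the rotation finishes.
; A DoOnce blocks re-entry until Reset is called.
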(event Custom|EnterCamera
  (bind _camera (Variables|Default|GetCamera))
  (Utilities|FlowControl|DoOnce false
    (:Completed
      (bind _asplayer (Utilities|Casting|CastToPlayer (Game|GetPlayerCharacter 0)))
      (Default|PossessCamera _asplayer)
      (bind _output_get (Variables|Default|SetCameraLoc (Transformation|GetWorldLocation (Variables|/Game/Player/Player.Player_C|GetFirstPersonCamera _asplayer))))
      (Transformation|SetWorldLocation _camera _output_get false false)
      (bind _output_get_2 (Variables|Default|SetCameraRot (Transformation|GetWorldRotation (Variables|/Game/Player/Player.Player_C|GetFirstPersonCamera _asplayer))))
      (Transformation|SetWorldRotation _camera _output_get_2 false false)
      (Game|Player|SetViewTargetwithBlend (Game|GetPlayerController 0) self 0.0 "VTBlend_Linear" 0.0 false)
      (Utilities|FlowControl|Delay 0.25)
      (Utilities|FlowControl|Sequence
        (:then_0
          (bind _newtrack_0 (Timeline|Timeline_0 PlayFromStart)
            (:Update
              (Transformation|SetWorldLocation (Variables|Default|GetCamera) (Math|Vector|Lerp(Vector) (Variables|Default|GetCameraLoc) "780.000000,-22.000000,364.000000" _newtrack_0) false false))))
        (:then_1
          (bind _newtrack_0_2 (Timeline|Timeline_1 PlayFromStart)
            (:Update
              (Transformation|SetWorldRotation (Variables|Default|GetCamera) (Math|Rotator|Lerp(Rotator) (Variables|Default|GetCameraRot) "0,-20.000000, 0" _newtrack_0_2 true) false false))
            (:Finished
              (Variables|Default|SetActive? true))))))))

(event Custom|Reset
  (bind _camera (Variables|Default|GetCamera))
  (Utilities|FlowControl|DoOnce false) ; enters at Reset
)

(fn ConstructionScript)

(fn Interact
  (CallFunction|EnterCamera)
  (return true))