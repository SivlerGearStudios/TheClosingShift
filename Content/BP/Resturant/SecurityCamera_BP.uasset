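; Security camera actor for the restaurant that jumps between five preset locations.
; MoveUp and MoveDown custom events step LocIndex forward or back, wrapping between 1 and 5.
; A switch on the index then sets the actor to the matching Loc variable without sweep.
; Both events also print a debug index value, offset one step from the new index.
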(event Custom|MoveUp
  (bind _output_get (Variables|Default|SetLocIndex (+ (Variables|Default|GetLocIndex) 1)))
  (Development|PrintString (Utilities|String|ToString(Integer) (+ (Variables|Default|GetLocIndex) 1)))
  (if (== _output_get 6)
    (Variables|Default|SetLocIndex 1))
  (switch int (Variables|Default|GetLocIndex)
    (:1
      (Transformation|SetActorLocation (Variables|Default|GetLoc1) false false))
    (:2
      (Transformation|SetActorLocation (Variables|Default|GetLoc2) false false))
    (:3
      (Transformation|SetActorLocation (Variables|Default|GetLoc3) false false))
    (:4
      (Transformation|SetActorLocation (Variables|Default|GetLoc4) false false))
    (:5
      (Transformation|SetActorLocation (Variables|Default|GetLoc5) false false))))

(event Custom|MoveDown
  (bind _output_get (Variables|Default|SetLocIndex (- (Variables|Default|GetLocIndex) 1)))
  (Development|PrintString (Utilities|String|ToString(Integer) (- (Variables|Default|GetLocIndex) 1)))
  (if (== _output_get 0)
    (Variables|Default|SetLocIndex 5))
  (switch int (Variables|Default|GetLocIndex)
    (:1
      (Transformation|SetActorLocation (Variables|Default|GetLoc1) false false))
    (:2
      (Transformation|SetActorLocation (Variables|Default|GetLoc2) false false))
    (:3
      (Transformation|SetActorLocation (Variables|Default|GetLoc3) false false))
    (:4
      (Transformation|SetActorLocation (Variables|Default|GetLoc4) false false))
    (:5
      (Transformation|SetActorLocation (Variables|Default|GetLoc5) false false))))

(fn ConstructionScript)