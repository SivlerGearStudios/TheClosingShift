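; BP_Hatchback is a drivable hatchback vehicle pawn with a player look camera and toggleable lights.
; Movement axes feed throttle and steering into VehicleMovement, while the F key switches two spotlights on or off through custom events tracked by LightsOn.
; Mouse look drives controller pitch and yaw, with pitch limited on the camera manager at BeginPlay and yaw nudged back when the camera's relative yaw passes its side limits.
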(event Custom|TurnOnLight
  (Rendering|Components|Light|SetIntensity (Variables|Default|GetSpotLight) 5e+04)
  (Rendering|Components|Light|SetIntensity (Variables|Default|GetSpotLight1) 5e+04)
  (Variables|Default|SetLightsOn? true))

(event Custom|TurnOffLights
  (Rendering|Components|Light|SetIntensity (Variables|Default|GetSpotLight) 0.0)
  (Rendering|Components|Light|SetIntensity (Variables|Default|GetSpotLight1) 0.0)
  (Variables|Default|SetLightsOn? false))

(event EventBeginPlay
  (bind _returnvalue (Game|GetPlayerCameraManager 0))
  (Variables|/Script/Engine.PlayerCameraManager|SetViewPitchMax _returnvalue 5e+01)
  (Variables|/Script/Engine.PlayerCameraManager|SetViewPitchMin _returnvalue -5e+01))

(event Input|AxisEvents|InputAxisMoveForward
  (params (AxisValue :type Float%20%28single-precision%29))
  (Class|WheeledVehicleMovementComponent|SetThrottleInput (Variables|Default|GetVehicleMovement) AxisValue))

(event Input|AxisEvents|InputAxisMoveRight
  (params (AxisValue :type Float%20%28single-precision%29))
  (Class|WheeledVehicleMovementComponent|SetSteeringInput (Variables|Default|GetVehicleMovement) AxisValue))

(event Input|AxisEvents|InputAxisLookUp
  (params (AxisValue :type Float%20%28single-precision%29))
  (Pawn|Input|AddControllerPitchInput AxisValue))

(event Input|AxisEvents|InputAxisTurn
  (params (AxisValue :type Float%20%28single-precision%29))
  (bind _camera (Variables|Default|GetCamera))
  (bind _relativerotation (Variables|/Script/Engine.SceneComponent|GetRelativeRotation _camera))
  (if (< (.yaw _relativerotation) -8e+01)
    (Pawn|Input|AddControllerYawInput 0.1)
    (elif (> (.yaw _relativerotation) 8e+01)
      (Pawn|Input|AddControllerYawInput -0.1)
      (else
        (Pawn|Input|AddControllerYawInput AxisValue)))))

(event Input|KeyboardEvents|F
  (params (Key :type Key%20Structure))
  (:Pressed
    (if (Variables|Default|GetLightsOn?)
      (CallFunction|TurnOffLights)
      (else
        (CallFunction|TurnonLight)))))

(fn ConstructionScript)